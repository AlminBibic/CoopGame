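; Player pawn Blueprint that handles a dance emote and creates the local player's HUD.
; The Dance input sets IsDancing and plays a Gangnam Style animation, then restores the Animation Blueprint and clears the flag after a fixed delay.
; Left click or W cuts the animation short through a shared DoOnce, reset on release, without clearing IsDancing.
; BeginPlay adds crosshair and health indicator widgets if locally controlled.
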(event `Key|LeftMouseButton`
  (params (Key :type "Key Structure"))
  ;[1 1 1] Handle Dance Animation
  (:`Pressed`
    (`/Engine/EditorBlueprintResources/StandardMacros.DoOnce` false :!label _label
      (:`Completed`
        (`SkeletalMeshComponent.SetAnimationMode` (`self.Mesh`) "AnimationBlueprint"))))
  (:`Released`
    (goto _label :!via `Reset`)))

(event `Key|W`
  (params (Key :type "Key Structure"))
  ;[1 1 1] Handle Dance Animation
  (:`Pressed`
    (goto _label))
  (:`Released`
    (goto _label :!via `Reset`)))

(event `InputAction|Dance`
  (params (Key :type "Key Structure"))
  ;[1 1 1] Handle Dance Animation
  (:`Pressed`
    (set `self.IsDancing` true)
    (`SkeletalMeshComponent.PlayAnimation` (`self.Mesh`) "/Game/Gangnam_Style_Anim_mixamo_com1.Gangnam_Style_Anim_mixamo_com1" false)
    (`KismetSystemLibrary.Delay` 12.367)
    (`SkeletalMeshComponent.SetAnimationMode` (`self.Mesh`) "AnimationBlueprint")
    (set `self.IsDancing` false)))

(event `self.ReceiveBeginPlay`
  (if (`self.IsLocallyControlled`)
    (`|ExecutionSequence`
      (:`then_0`
        (bind _returnvalue (`|CreateWidget` "/Game/UI/WBP_Crosshair.WBP_Crosshair_C"))
        (`UserWidget.AddToViewport` _returnvalue 0))
      (:`then_1`
        (bind _returnvalue_2 (`|CreateWidget` "/Game/UI/WBP_HealthIdicator.WBP_HealthIdicator_C"))
        (`UserWidget.AddToViewport` _returnvalue_2 0)))))

(fn `UserConstructionScript`)